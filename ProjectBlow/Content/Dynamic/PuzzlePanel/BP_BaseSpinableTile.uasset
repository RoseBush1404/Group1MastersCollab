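; BP_BaseSpinableTile is a base puzzle-panel tile that spins a quarter turn in yaw each time RotateTile is called.
; A timeline lerps the root's relative rotation, and an IsRotating flag ignores calls made mid-spin.
; The construction script disables collision on North, South, East and West colliders whose connection-point flag is off.
; Overlap events exist only for the North collider and just print debug messages.
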(event `/Game/Dynamic/PuzzlePanel/iTileInput.RotateTile`
  (bind _startingrotation (`self.StartingRotation`))
  (if (not (`self.IsRotating`))
    (set `self.IsRotating` true)
    (set `self.StartingRotation` (`SceneComponent.RelativeRotation` (`self.DefaultSceneRoot`)))
    (bind (_direction _alpha) (`Timeline|RotateTileTimeLine` :!via `PlayFromStart`)
      (:`Update`
        (`SceneComponent.K2_SetRelativeRotation` (`self.DefaultSceneRoot`) (`KismetMathLibrary.RLerp` _startingrotation (`KismetMathLibrary.MakeRotator` (.roll _startingrotation) (.pitch _startingrotation) (+ (.yaw _startingrotation) 90.0)) _alpha) false false))
      (:`Finished`
        (set `self.IsRotating` false)))))

(event `self.NorthCollider.OnComponentBeginOverlap`
  (params (OverlappedComponent :type "PrimitiveComponent Object Reference") (OtherActor :type "Actor Object Reference") (OtherComp :type "PrimitiveComponent Object Reference") (OtherBodyIndex :type Integer) (bFromSweep :type Boolean) (SweepResult :type "HitResult Structure (by ref)"))
  (`KismetSystemLibrary.PrintString` "North Has Triggered"))

(event `self.NorthCollider.OnComponentEndOverlap`
  (params (OverlappedComponent :type "PrimitiveComponent Object Reference") (OtherActor :type "Actor Object Reference") (OtherComp :type "PrimitiveComponent Object Reference") (OtherBodyIndex :type Integer))
  (`KismetSystemLibrary.PrintString` "North is no longer Triggered"))

(fn `UserConstructionScript`
  (`|ExecutionSequence`
    (:`then_0`
      (if (not (`self.HasNorthPoint`))
        (`PrimitiveComponent.SetCollisionEnabled` (`self.NorthCollider`) "NoCollision")))
    (:`then_1`
      (if (not (`self.HasSouthPoint`))
        (`PrimitiveComponent.SetCollisionEnabled` (`self.SouthCollider`) "NoCollision")))
    (:`then_2`
      (if (not (`self.HasEastPoint`))
        (`PrimitiveComponent.SetCollisionEnabled` (`self.EastCollider`) "NoCollision")))
    (:`then_3`
      (if (not (`self.HasWestPoint`))
        (`PrimitiveComponent.SetCollisionEnabled` (`self.WestCollider`) "NoCollision")))))