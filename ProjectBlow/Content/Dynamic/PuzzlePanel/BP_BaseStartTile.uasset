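; Base Blueprint for the start tile of a tile-connection puzzle panel, acting as an always-powered tile.
; Overlaps on its North collider add and remove neighbouring tiles in a unique Connections list, resolved through a tile-reference message call.
; Getter functions expose that list and return itself as both tile actor and start tile, while the end and spinable tile getters return nothing.
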(event `self.NorthCollider.OnComponentBeginOverlap`
  (params (OverlappedComponent :type "PrimitiveComponent Object Reference") (OtherActor :type "Actor Object Reference") (OtherComp :type "PrimitiveComponent Object Reference") (OtherBodyIndex :type Integer) (bFromSweep :type Boolean) (SweepResult :type "HitResult Structure (by ref)"))
  (`self.AddConnection` OtherActor))

(event `self.NorthCollider.OnComponentEndOverlap`
  (params (OverlappedComponent :type "PrimitiveComponent Object Reference") (OtherActor :type "Actor Object Reference") (OtherComp :type "PrimitiveComponent Object Reference") (OtherBodyIndex :type Integer))
  (`self.RemoveConnection` OtherActor))

(fn `AddConnection`
  (params (`Other Actor` :type "Object Object Reference"))
  (bind _actorref (message `/Game/Dynamic/PuzzlePanel/iTileInput.GetTileActorRef` `Other Actor`))
  (`/Engine/EditorBlueprintResources/StandardMacros.IsValid` _actorref
    (:`Is Valid`
      (`KismetArrayLibrary.Array_AddUnique` (`self.Connections`) _actorref))))

(fn `GetAllConnections`
  (returns (Connections :type "Array of Actor Object Reference"))
  (return (`self.Connections`)))

(fn `GetEndTileRef`
  (returns (EndTileRef :type "/Game/Dynamic/PuzzlePanel/BP_BaseEndTile Object Reference"))
  (return null))

(fn `GetIsPowered`
  (returns (IsPowered :type Boolean))
  (return true))

(fn `GetSpinableTileRef`
  (returns (`Tile Ref` :type "/Game/Dynamic/PuzzlePanel/BP_BaseSpinableTile Object Reference"))
  (return null))

(fn `GetStartTileRef`
  (returns (StartTileRef :type "/Game/Dynamic/PuzzlePanel/BP_BaseStartTile Object Reference"))
  (return self))

(fn `GetTileActorRef`
  (returns (ActorRef :type "Actor Object Reference"))
  (return self))

(fn `RemoveConnection`
  (params (`Other Actor` :type "Object Object Reference"))
  (bind _actorref (message `/Game/Dynamic/PuzzlePanel/iTileInput.GetTileActorRef` `Other Actor`))
  (`KismetArrayLibrary.Array_RemoveItem` (`self.Connections`) _actorref))

(fn `UserConstructionScript`)