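; Base end tile for a puzzle panel, acting as an endpoint that can be powered up or down.
; Overlaps on its north collider add or remove neighboring tile actors in a Connections list, resolved through interface messages.
; Powering up turns the point light green and fires an end-powered-up event, while powering down turns it red.
; Getters expose connections, power state and itself, with spinnable and start tile getters returning empty.
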(event `self.NorthCollider.OnComponentBeginOverlap`
  (params (OverlappedComponent :type "PrimitiveComponent Object Reference") (OtherActor :type "Actor Object Reference") (OtherComp :type "PrimitiveComponent Object Reference") (OtherBodyIndex :type Integer) (bFromSweep :type Boolean) (SweepResult :type "HitResult Structure (by ref)"))
  (`self.AddConnection` OtherActor))

(event `/Game/Dynamic/PuzzlePanel/iTileInput.PowerUp`
  (`LightComponent.SetLightColor` (`self.PointLight`) (struct :`G` 1.0 :`A` 1.0) true)
  (set `self.IsPowered` true)
  (`self.OnEndPoweredUp`))

(event `self.NorthCollider.OnComponentEndOverlap`
  (params (OverlappedComponent :type "PrimitiveComponent Object Reference") (OtherActor :type "Actor Object Reference") (OtherComp :type "PrimitiveComponent Object Reference") (OtherBodyIndex :type Integer))
  (`self.RemoveConnection` OtherActor))

(event `/Game/Dynamic/PuzzlePanel/iTileInput.PowerDown`
  (`LightComponent.SetLightColor` (`self.PointLight`) (struct :`R` 1.0 :`G` 0.016 :`A` 1.0) true)
  (set `self.IsPowered` false))

(fn `AddConnection`
  (params (`Other Actor` :type "Object Object Reference"))
  (bind _actorref (message `/Game/Dynamic/PuzzlePanel/iTileInput.GetTileActorRef` `Other Actor`))
  (`/Engine/EditorBlueprintResources/StandardMacros.IsValid` _actorref
    (:`Is Valid`
      (`KismetArrayLibrary.Array_AddUnique` (`self.Connections`) _actorref))))

(fn `GetAllConnections`
  (returns (Connections :type "Array of Actor Object Reference"))
  (return (`self.Connections`)))

(fn `GetEndTileRef`
  (returns (EndTileRef :type "/Game/Dynamic/PuzzlePanel/BP_BaseEndTile Object Reference"))
  (return self))

(fn `GetIsPowered`
  (returns (IsPowered :type Boolean))
  (return (`self.IsPowered`)))

(fn `GetSpinableTileRef`
  (returns (`Tile Ref` :type "/Game/Dynamic/PuzzlePanel/BP_BaseSpinableTile Object Reference"))
  (return null))

(fn `GetStartTileRef`
  (returns (StartTileRef :type "/Game/Dynamic/PuzzlePanel/BP_BaseStartTile Object Reference"))
  (return null))

(fn `GetTileActorRef`
  (returns (ActorRef :type "Actor Object Reference"))
  (return self))

(fn `RemoveConnection`
  (params (`Other Actor` :type "Object Object Reference"))
  (bind _actorref (message `/Game/Dynamic/PuzzlePanel/iTileInput.GetTileActorRef` `Other Actor`))
  (`KismetArrayLibrary.Array_RemoveItem` (`self.Connections`) _actorref))

(fn `UserConstructionScript`)