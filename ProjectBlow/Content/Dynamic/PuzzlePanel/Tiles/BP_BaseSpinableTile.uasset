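; Base spinnable tile for a puzzle panel that rotates to link with other tiles and shows powered state by swapping materials.
; Four directional colliders, disabled at construction where the tile has no connection point, maintain the Connections list through overlap events.
; Timelines lerp 90-degree yaw turns or resets to the spawn rotation with a Z offset, guarded by IsRotating, then call CallOnFinishRotating.
; Getters expose connections, power state and tile references.
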(event `self.NorthCollider.OnComponentBeginOverlap`
  (params (OverlappedComponent :type "PrimitiveComponent Object Reference") (OtherActor :type "Actor Object Reference") (OtherComp :type "PrimitiveComponent Object Reference") (OtherBodyIndex :type Integer) (bFromSweep :type Boolean) (SweepResult :type "HitResult Structure (by ref)"))
  ;[1 1 1] Collision Dection
  (`self.AddConnection` OtherActor))

(event `/Game/Dynamic/PuzzlePanel/iTileInput.PowerUp`
  ;[1 1 1] Power Up/Down
  (`PrimitiveComponent.SetMaterial` (`self.StaticMesh`) 1 (`self.PowerUpMaterial`))
  (set `self.IsPowered` true))

(event `/Game/Dynamic/PuzzlePanel/iTileInput.RotateTile`
  (bind _defaultsceneroot (`self.DefaultSceneRoot`))
  (bind _startingrotation (`self.StartingRotation`))
  (bind _startinglocation (`self.StartingLocation`))
  (bind _defaultsceneroot_2 (`self.DefaultSceneRoot`))
  ;[1 1 1] Rotate Tile
  (if (not (`self.IsRotating`))
    (set `self.IsRotating` true)
    (set `self.StartingRotation` (`SceneComponent.RelativeRotation` _defaultsceneroot))
    (set `self.StartingLocation` (`SceneComponent.RelativeLocation` _defaultsceneroot))
    (bind (_direction _rotationalpha _locationalpha) (`Timeline|RotateTileTimeLine` :!via `PlayFromStart`)
      (:`Update`
        (`SceneComponent.K2_SetRelativeRotation` _defaultsceneroot_2 (`KismetMathLibrary.RLerp` _startingrotation (`KismetMathLibrary.MakeRotator` (.roll _startingrotation) (.pitch _startingrotation) (+ (.yaw _startingrotation) 90.0)) _rotationalpha) false false)
        (`SceneComponent.K2_SetRelativeLocation` _defaultsceneroot_2 (`KismetMathLibrary.VLerp` _startinglocation (`KismetMathLibrary.MakeVector` (.x _startinglocation) (.y _startinglocation) (+ (.z _startinglocation) 10.0)) _locationalpha) false false))
      (:`Finished`
        (set `self.IsRotating` false)
        (`self.OnFinishRotating`))
      (:`SoundTrigger`
        (`self.RotationSFX`)))))

(event `/Game/Dynamic/PuzzlePanel/iTileInput.PowerDown`
  ;[1 1 1] Power Up/Down
  (`PrimitiveComponent.SetMaterial` (`self.StaticMesh`) 1 (`self.PowerDownMaterial`))
  (set `self.IsPowered` false))

(event `self.NorthCollider.OnComponentEndOverlap`
  (params (OverlappedComponent :type "PrimitiveComponent Object Reference") (OtherActor :type "Actor Object Reference") (OtherComp :type "PrimitiveComponent Object Reference") (OtherBodyIndex :type Integer))
  ;[1 1 1] Collision Dection
  (`self.RemoveConnection` OtherActor))

(event `self.SouthCollider.OnComponentBeginOverlap`
  (params (OverlappedComponent :type "PrimitiveComponent Object Reference") (OtherActor :type "Actor Object Reference") (OtherComp :type "PrimitiveComponent Object Reference") (OtherBodyIndex :type Integer) (bFromSweep :type Boolean) (SweepResult :type "HitResult Structure (by ref)"))
  ;[1 1 1] Collision Dection
  (`self.AddConnection` OtherActor))

(event `self.SouthCollider.OnComponentEndOverlap`
  (params (OverlappedComponent :type "PrimitiveComponent Object Reference") (OtherActor :type "Actor Object Reference") (OtherComp :type "PrimitiveComponent Object Reference") (OtherBodyIndex :type Integer))
  ;[1 1 1] Collision Dection
  (`self.RemoveConnection` OtherActor))

(event `self.WestCollider.OnComponentBeginOverlap`
  (params (OverlappedComponent :type "PrimitiveComponent Object Reference") (OtherActor :type "Actor Object Reference") (OtherComp :type "PrimitiveComponent Object Reference") (OtherBodyIndex :type Integer) (bFromSweep :type Boolean) (SweepResult :type "HitResult Structure (by ref)"))
  ;[1 1 1] Collision Dection
  (`self.AddConnection` OtherActor))

(event `self.ReceiveBeginPlay`
  ;[1 1 1] Reset
  (`KismetSystemLibrary.Delay` 0.3)
  (set `self.SpawnedRotation` (`SceneComponent.RelativeRotation` (`self.DefaultSceneRoot`))))

(event `self.WestCollider.OnComponentEndOverlap`
  (params (OverlappedComponent :type "PrimitiveComponent Object Reference") (OtherActor :type "Actor Object Reference") (OtherComp :type "PrimitiveComponent Object Reference") (OtherBodyIndex :type Integer))
  ;[1 1 1] Collision Dection
  (`self.RemoveConnection` OtherActor))

(event `/Game/Dynamic/PuzzlePanel/iTileInput.ResetTile`
  (bind _defaultsceneroot (`self.DefaultSceneRoot`))
  (bind _defaultsceneroot_2 (`self.DefaultSceneRoot`))
  (bind _startinglocation (`self.StartingLocation`))
  ;[1 1 1] Reset
  (if (not (`self.IsRotating`))
    (set `self.IsRotating` true)
    (set `self.StartingRotation` (`SceneComponent.RelativeRotation` _defaultsceneroot_2))
    (set `self.StartingLocation` (`SceneComponent.RelativeLocation` _defaultsceneroot_2))
    (bind (_direction _rotationalpha _locationalpha) (`Timeline|ResetTileTimeLine` :!via `PlayFromStart`)
      (:`Update`
        (`SceneComponent.K2_SetRelativeRotation` _defaultsceneroot (`KismetMathLibrary.RLerp` (`self.StartingRotation`) (`self.SpawnedRotation`) _rotationalpha) false false)
        (`SceneComponent.K2_SetRelativeLocation` _defaultsceneroot (`KismetMathLibrary.VLerp` _startinglocation (`KismetMathLibrary.MakeVector` (.x _startinglocation) (.y _startinglocation) (+ (.z _startinglocation) 10.0)) _locationalpha) false false))
      (:`Finished`
        (set `self.IsRotating` false)
        (`self.OnFinishRotating`)))))

(event `self.EastCollider.OnComponentBeginOverlap`
  (params (OverlappedComponent :type "PrimitiveComponent Object Reference") (OtherActor :type "Actor Object Reference") (OtherComp :type "PrimitiveComponent Object Reference") (OtherBodyIndex :type Integer) (bFromSweep :type Boolean) (SweepResult :type "HitResult Structure (by ref)"))
  ;[1 1 1] Collision Dection
  (`self.AddConnection` OtherActor))

(event `self.EastCollider.OnComponentEndOverlap`
  (params (OverlappedComponent :type "PrimitiveComponent Object Reference") (OtherActor :type "Actor Object Reference") (OtherComp :type "PrimitiveComponent Object Reference") (OtherBodyIndex :type Integer))
  ;[1 1 1] Collision Dection
  (`self.RemoveConnection` OtherActor))

(fn `AddConnection`
  (params (`Other Actor` :type "Object Object Reference"))
  (bind _actorref (message `/Game/Dynamic/PuzzlePanel/iTileInput.GetTileActorRef` `Other Actor`))
  (`/Engine/EditorBlueprintResources/StandardMacros.IsValid` _actorref
    (:`Is Valid`
      (`KismetArrayLibrary.Array_AddUnique` (`self.Connections`) _actorref))))

(fn `GetAllConnections`
  (returns (Connections :type "Array of Actor Object Reference"))
  (return (`self.Connections`)))

(fn `GetEndTileRef`
  (returns (EndTileRef :type "/Game/Dynamic/PuzzlePanel/Tiles/BP_BaseEndTile Object Reference"))
  (return null))

(fn `GetIsPowered`
  (returns (IsPowered :type Boolean))
  (return (`self.IsPowered`)))

(fn `GetSpinableTileRef`
  (returns (`Tile Ref` :type "/Game/Dynamic/PuzzlePanel/Tiles/BP_BaseSpinableTile Object Reference"))
  (return self))

(fn `GetStartTileRef`
  (returns (StartTileRef :type "/Game/Dynamic/PuzzlePanel/Tiles/BP_BaseStartTile Object Reference"))
  (return null))

(fn `GetTileActorRef`
  (returns (ActorRef :type "Actor Object Reference"))
  (return self))

(fn `GetTileRef`
  (returns (`Tile Ref` :type "/Game/Dynamic/PuzzlePanel/Tiles/BP_BaseSpinableTile Object Reference"))
  (return self))

(fn `RemoveConnection`
  (params (`Other Actor` :type "Object Object Reference"))
  (bind _actorref (message `/Game/Dynamic/PuzzlePanel/iTileInput.GetTileActorRef` `Other Actor`))
  (`KismetArrayLibrary.Array_RemoveItem` (`self.Connections`) _actorref))

(fn `RotationSFX`
  (`GameplayStatics.PlaySoundAtLocation` "/Game/Static/Audio/PuzzlePanel/SC_TileRotation.SC_TileRotation" (`self.K2_GetActorLocation`) (struct) 1.0 1.0 0.0 null null null))

(fn `UserConstructionScript`
  (`|ExecutionSequence`
    (:`then_0`
      (if (not (`self.HasNorthPoint`))
        (`PrimitiveComponent.SetCollisionEnabled` (`self.NorthCollider`) "NoCollision")))
    (:`then_1`
      (if (not (`self.HasSouthPoint`))
        (`PrimitiveComponent.SetCollisionEnabled` (`self.SouthCollider`) "NoCollision")))
    (:`then_2`
      (if (not (`self.HasEastPoint`))
        (`PrimitiveComponent.SetCollisionEnabled` (`self.EastCollider`) "NoCollision")))
    (:`then_3`
      (if (not (`self.HasWestPoint`))
        (`PrimitiveComponent.SetCollisionEnabled` (`self.WestCollider`) "NoCollision")))))