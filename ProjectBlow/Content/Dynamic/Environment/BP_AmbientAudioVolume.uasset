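; BP_AmbientAudioVolume is a box trigger volume that fades a referenced ambient sound to a set volume when the player character enters it.
; On overlap it records the audio component's current volume multiplier and, if that differs from the target, plays a timeline that lerps between the two.
; The construction script sizes the box from an extent variable.
; Nothing reverts the volume on exit.
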(event `self.Box.OnComponentBeginOverlap`
  (params (OverlappedComponent :type "PrimitiveComponent Object Reference") (OtherActor :type "Actor Object Reference") (OtherComp :type "PrimitiveComponent Object Reference") (OtherBodyIndex :type Integer) (bFromSweep :type Boolean) (SweepResult :type "HitResult Structure (by ref)"))
  (bind _ambientaudioref (`self.AmbientAudioRef`))
  (bind _audiocomponent (`AmbientSound.AudioComponent` _ambientaudioref))
  (if (== OtherActor (`GameplayStatics.GetPlayerCharacter` 0))
    (`/Engine/EditorBlueprintResources/StandardMacros.IsValid` _ambientaudioref
      (:`Is Valid`
        (bind _output_get (set `self.StartingVolume` (`AudioComponent.VolumeMultiplier` _audiocomponent)))
        (if (!= _output_get (`self.VolumeMultiplier`))
          (bind (_direction _alpha) (`Timeline|VolumeTransition` :!via `PlayFromStart`)
            (:`Update`
              (`AudioComponent.SetVolumeMultiplier` _audiocomponent (`KismetMathLibrary.Lerp` (`self.StartingVolume`) (`self.VolumeMultiplier`) _alpha)))))))))

(fn `UserConstructionScript`
  (`BoxComponent.SetBoxExtent` (`self.Box`) (`self.VolumeExtent`) true))