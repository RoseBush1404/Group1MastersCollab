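; BP_BaseDoor is a base door that reacts when its connected puzzle panel is completed.
; On BeginPlay it binds to the panel's completion event, if a panel is assigned.
; Completion waits a configurable delay, then calls StartDoorMovment and plays a grinding sound at the door's location with adjustable volume and pitch.
; StartDoorMovment is empty here, so this Blueprint defines no movement itself.
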(event `self.ReceiveBeginPlay`
  (bind _connectedpuzzlepanel (`self.ConnectedPuzzlePanel`))
  (`/Engine/EditorBlueprintResources/StandardMacros.IsValid` _connectedpuzzlepanel
    (:`Is Valid`
      (add `/Game/Dynamic/PuzzlePanel/Puzzles/BasePuzzlePanel.OnPuzzleIsCompleted` _connectedpuzzlepanel (`|CreateDelegate` :!event `PuzzleCompleted`)))))

(event `PuzzleCompleted`
  (params (Puzzle :type "/Game/Dynamic/PuzzlePanel/Puzzles/BasePuzzlePanel Object Reference"))
  (`KismetSystemLibrary.Delay` (`self.CompletionDelay`))
  (`self.StartDoorMovment`)
  (`self.PlayDoorSound`))

(event `StartDoorMovment`)

(fn `PlayDoorSound`
  (returns (Ignore :type Boolean))
  (`GameplayStatics.PlaySoundAtLocation` "/Game/Static/Audio/Environment/StoneGrinding/Grinding_5.Grinding_5" (`self.K2_GetActorLocation`) (struct) (`self.DoorSFXVolume`) (`self.DoorSFXPitch`) 0.0 null null null)
  (return false))

(fn `UserConstructionScript`)