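; BP_FinalGates is a double-door gate that swings both leaves open in opposite yaw directions, extending a parent door Blueprint.
; StartDoorMovment caches each pivot's world rotation, then a timeline lerps the left pivot by plus RotationAmount and the right by minus RotationAmount.
; PlayDoorSound calls the parent, then plays DoorSFX at the actor's location with configurable volume and pitch.
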(event `self.StartDoorMovment`
  (bind _leftdoorstartingrotation (`self.LeftDoorStartingRotation`))
  (bind _rightdoorstartingrotation (`self.RightDoorStartingRotation`))
  (set `self.LeftDoorStartingRotation` (`SceneComponent.K2_GetComponentRotation` (`self.LeftDoorPivit`)))
  (set `self.RightDoorStartingRotation` (`SceneComponent.K2_GetComponentRotation` (`self.RightDoorPivit`)))
  (bind (_direction _alpha) (`Timeline|Timeline_0` :!via `PlayFromStart`)
    (:`Update`
      (`SceneComponent.K2_SetWorldRotation` (`self.LeftDoorPivit`) (`KismetMathLibrary.RLerp` _leftdoorstartingrotation (`KismetMathLibrary.MakeRotator` (.roll _leftdoorstartingrotation) (.pitch _leftdoorstartingrotation) (+ (.yaw _leftdoorstartingrotation) (`self.RotationAmount`))) _alpha) false false)
      (`SceneComponent.K2_SetWorldRotation` (`self.RightDoorPivit`) (`KismetMathLibrary.RLerp` _rightdoorstartingrotation (`KismetMathLibrary.MakeRotator` (.roll _rightdoorstartingrotation) (.pitch _rightdoorstartingrotation) (- (.yaw _rightdoorstartingrotation) (`self.RotationAmount`))) _alpha) false false))))

(fn `PlayDoorSound`
  (returns (Ignore :type Boolean))
  (`parent.PlayDoorSound`)
  (`GameplayStatics.PlaySoundAtLocation` (`self.DoorSFX`) (`self.K2_GetActorLocation`) (struct) (`self.DoorSFXVolume`) (`self.DoorSFXPitch`) 0.0 null null null)
  (return false))

(fn `UserConstructionScript`
  (`parent.UserConstructionScript`))