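; Basement door Blueprint that slides its Door component to an offset position when the StartDoorMovment event is called.
; The event caches the door's world location, then plays the DoorMovement timeline from the start.
; Each timeline update lerps the location toward the start plus EndLocation, so EndLocation acts as a world-space offset, and moves without sweeping.
; The file contains no trigger or closing logic, and the construction script only calls its parent.
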(event `self.StartDoorMovment`
  (bind _startlocation (`self.StartLocation`))
  (set `self.StartLocation` (`SceneComponent.K2_GetComponentLocation` (`self.Door`)))
  (bind (_direction _aphla) (`Timeline|DoorMovement` :!via `PlayFromStart`)
    (:`Update`
      (`SceneComponent.K2_SetWorldLocation` (`self.Door`) (`KismetMathLibrary.VLerp` _startlocation (+ _startlocation (`self.EndLocation`)) _aphla) false false))))

(fn `UserConstructionScript`
  (`parent.UserConstructionScript`))